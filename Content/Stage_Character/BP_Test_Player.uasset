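; BP_Test_Player is a test player Blueprint used to print debug values on key presses.
; Keys 1, 2 and 3 each print one of three variables, TestVec1 to TestVec3, as a string.
; BeginPlay, Tick and the construction script are empty, and nothing in these graphs sets the variables.
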(event `Key|One`
  (params (Key :type "Key Structure"))
  (:`Pressed`
    (`KismetSystemLibrary.PrintString` (`KismetStringLibrary.Conv_VectorToString` (`self.TestVec1`)))))

(event `Key|Two`
  (params (Key :type "Key Structure"))
  (:`Pressed`
    (`KismetSystemLibrary.PrintString` (`KismetStringLibrary.Conv_VectorToString` (`self.TestVec2`)))))

(event `Key|Three`
  (params (Key :type "Key Structure"))
  (:`Pressed`
    (`KismetSystemLibrary.PrintString` (`KismetStringLibrary.Conv_VectorToString` (`self.TestVec3`)))))

(fn `UserConstructionScript`)