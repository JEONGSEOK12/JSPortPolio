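; BP_Stage_Plane_2 is a stage select map trigger that gates entry to Stage 2.
; When an actor tagged Player overlaps it, it reads ClearLevel from BP_MyGameInstance.
; At 1 or higher, it sets ClearLevel to 2 before opening Stage_2_Test, so the value changes on entry rather than on completion.
; Otherwise it prints a message that Level 1 must be cleared.
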(event `self.ReceiveActorBeginOverlap`
  (params (OtherActor :type "Actor Object Reference"))
  (if (`self.ActorHasTag` OtherActor "Player")
    (bind _asbp_my_game_instance (cast `/Game/BP_MyGameInstance` (`GameplayStatics.GetGameInstance`)))
    (if (>= (`MyGameInstance.ClearLevel` _asbp_my_game_instance) 1)
      (bind _asbp_my_game_instance_2 (cast `/Game/BP_MyGameInstance` (`GameplayStatics.GetGameInstance`)))
      (set `MyGameInstance.ClearLevel` 2 _asbp_my_game_instance_2)
      (`GameplayStatics.OpenLevelBySoftObjectPtr` "/Game/Levels/Not_Test/Stage_2_Test.Stage_2_Test")
      (else
        (`KismetSystemLibrary.PrintString` "Must Clear Level 1")))))

(fn `UserConstructionScript`)